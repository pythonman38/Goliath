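; Base enemy character Blueprint that handles the death sequence: freezing animation, disabling capsule collision and dissolving the enemy.
; OnEnemyDied caches the equipped weapon, then async-loads a Niagara effect, attaches it to the mesh and tints it with the material's dissolve edge color.
; A timeline scaled to TotalDissolveTime drives DissolveAmount on body and weapon, both only while the weapon is valid, then destroys them.
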(event Custom|DsiableAnimations
  (Variables|/Script/Engine.SkeletalMeshComponent|SetbPauseAnims (Variables|Character|GetMesh) true)
  (Collision|SetCollisionEnabled (Variables|Default|GetCapsuleComponent) "NoCollision"))

(event Custom|SpawnVFX_Material
  (bind _currentequippedweapon (Variables|Default|GetCurrentEquippedWeapon))
  (bind _currentequippedweapon_2 (Variables|Default|GetCurrentEquippedWeapon))
  (Components|Timeline|SetPlayRate (Variables|Default|GetDissolveTImeline) (/ 1.0 (Variables|Default|GetTotalDissolveTime)))
  (bind _normalizedfloattrack (Timeline|DissolveTImeline PlayFromStart)
    (:Update
      (bind _output_get (Variables|Default|SetFloatTrack _normalizedfloattrack))
      (Utilities|IsValid _currentequippedweapon_2
        (:Is%20Valid
          (Rendering|Material|SetScalarParameterValueonMaterials (Variables|/Script/Goliath.GoliathWeaponBase|GetWeaponMesh _currentequippedweapon_2) "DissolveAmount" _output_get)
          (Rendering|Material|SetScalarParameterValueonMaterials (Variables|Character|GetMesh) "DissolveAmount" (Variables|Default|GetFloatTrack)))))
    (:Finished
      (Utilities|IsValid _currentequippedweapon
        (:Is%20Valid
          (Actor|DestroyActor _currentequippedweapon))
        (:Is%20Not%20Valid
          _))
      (Actor|DestroyActor))))

(event Custom|SpawnVFX_Effects
  (params (Asset :type Object%20Soft%20Object%20Reference))
  (bind _mesh (Variables|Character|GetMesh))
  (bind _object (Utilities|AsyncLoadAsset Asset)
    (:Completed
      (bind _asniagara_system (Utilities|Casting|CastToNiagaraSystem _object))
      (bind _returnvalue (Niagara|SpawnSystemAttached _asniagara_system (Variables|Character|GetMesh) "None" "0, 0, 0" "0, 0, 0" "KeepRelativeOffset" true))
      (Variables|Default|SetNiagaraSystem _returnvalue)
      (bind _returnvalue_2 (Rendering|Material|CreateDynamicMaterialInstance _mesh 0 (Rendering|Material|GetMaterial _mesh 0) "None" :!class /Script/Engine.PrimitiveComponent))
      (bind _returnvalue_3 (Rendering|Material|GetVectorParameterValue _returnvalue_2 "DissolveEdgeColor" :!class /Script/Engine.MaterialInstanceDynamic))
      (Niagara|SetNiagaraVariable(LinearColor) (Variables|Default|GetNiagaraSystem) "DissolveParticleColor" _returnvalue_3))))

(event EventBeginPlay)

(event Collision|EventActorBeginOverlap
  (params (OtherActor :type Actor%20Object%20Reference)))

(event EventTick
  (params (DeltaSeconds :type Float%20%28single-precision%29)))

(event EventOnEnemyDied
  (params (DissolveNiagaraSystem :type Niagara%20System%20Soft%20Object%20Reference))
  (Variables|Default|SetCurrentEquippedWeapon (Class|PawnCombatComponent|GetCharacterCurrentEquippedWeapon (Variables|Default|GetEnemyCombatComponent)))
  (CallFunction|DsiableAnimations)
  (CallFunction|SpawnVFXEffects DissolveNiagaraSystem)
  (CallFunction|SpawnVFXMaterial))

(fn ConstructionScript)