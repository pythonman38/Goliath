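; Base projectile Blueprint that handles the audio and visual effects of a projectile's launch and impact.
; BeginPlay plays the spawn sound, attaches the flying sound to the root and spawns the Niagara muzzle effect facing forward.
; OnSpawnProjectileHitFX plays the impact sound and effect at the hit location, with the effect spawning only when the impact sound is also valid.
; Movement and hit detection are absent from these graphs.
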(event EventBeginPlay
  (bind _returnvalue (Transformation|GetActorLocation))
  (Audio|PlaySoundatLocation (Variables|Default|GetProjectileSpawnSound) _returnvalue "0, 0, 0" 1.0 1.0 0.0 0 0 0 0)
  (Audio|SpawnSoundAttached (Variables|Default|GetProjectileFlyingSound) (Variables|Transformation|GetRootComponent) "None" "0, 0, 0" "0, 0, 0" "KeepRelativeOffset" true 1.0 1.0 0.0 0 0)
  (Niagara|SpawnSystematLocation (Variables|Default|GetProjectileMuzzleFX) _returnvalue (Math|Conversions|RotationFromXVector (Transformation|GetActorForwardVector))))

(event EventOnSpawnProjectileHitFX
  (params (HitLocation :type Vector%20%28by%20ref%29 :default "0, 0, 0"))
  (bind _projectileimpactsound (Variables|Default|GetProjectileImpactSound)
    (:then
      (Audio|PlaySoundatLocation _projectileimpactsound HitLocation "0, 0, 0" 1.0 1.0 0.0 0 0 0 0)
      (bind _projectileimpactfx (Variables|Default|GetProjectileImpactFX)
        (:then
          (Niagara|SpawnSystematLocation _projectileimpactfx HitLocation))
        (:else)))
    (:else)))

(fn ConstructionScript)