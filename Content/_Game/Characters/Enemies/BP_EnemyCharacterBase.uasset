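; Base enemy character Blueprint that handles visual spawn and death presentation.
; On BeginPlay it reverses a timeline to un-dissolve the mesh and equipped weapon, and plays a random entry montage.
; On death it freezes animation, disables capsule collision and removes enemy widgets.
; It then async-loads a Niagara effect tinted from the material's dissolve edge color, while a timeline dissolves character and weapon before destroying both.
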(event Custom|DsiableAnimations
  (Variables|/Script/Engine.SkeletalMeshComponent|SetbPauseAnims (Variables|Character|GetMesh) true)
  (Variables|/Script/Engine.CharacterMovementComponent|SetbOrientRotationToMovement (Variables|Character|GetCharacterMovement) false)
  (Collision|SetCollisionEnabled (Variables|Default|GetCapsuleComponent) "NoCollision"))

(event Custom|SpawnVFX_Material
  (bind _currentequippedweapon (Variables|Default|GetCurrentEquippedWeapon))
  (bind _currentequippedweapon_2 (Variables|Default|GetCurrentEquippedWeapon))
  (Components|Timeline|SetPlayRate (Variables|Default|GetDissolveTImeline) (/ 1.0 (Variables|Default|GetTotalDissolveTime)))
  (bind _normalizedfloattrack (Timeline|DissolveTImeline PlayFromStart)
    (:Update
      (bind _output_get (Variables|Default|SetDissolveFloatTrack _normalizedfloattrack))
      (Utilities|IsValid _currentequippedweapon_2
        (:Is%20Valid
          (Rendering|Material|SetScalarParameterValueonMaterials (Variables|/Script/Goliath.GoliathWeaponBase|GetWeaponMesh _currentequippedweapon_2) "DissolveAmount" _output_get))
        (:Is%20Not%20Valid
          _))
      ;[0 0 0 0.5] Dissolve FX On Character
      (Rendering|Material|SetScalarParameterValueonMaterials (Variables|Character|GetMesh) "DissolveAmount" (Variables|Default|GetDissolveFloatTrack)))
    (:Finished
      (Utilities|IsValid _currentequippedweapon
        (:Is%20Valid
          (Actor|DestroyActor _currentequippedweapon))
        (:Is%20Not%20Valid
          _))
      (Actor|DestroyActor))))

(event Custom|SpawnVFX_Effects
  (params (Asset :type Object%20Soft%20Object%20Reference))
  (bind _mesh (Variables|Character|GetMesh))
  (bind _object (Utilities|AsyncLoadAsset Asset)
    (:Completed
      (bind _asniagara_system (Utilities|Casting|CastToNiagaraSystem _object))
      (bind _returnvalue (Niagara|SpawnSystemAttached _asniagara_system (Variables|Character|GetMesh) "None" "0, 0, 0" "0, 0, 0" "KeepRelativeOffset" true))
      (Variables|Default|SetNiagaraSystem _returnvalue)
      (bind _returnvalue_2 (Rendering|Material|CreateDynamicMaterialInstance _mesh 0 (Rendering|Material|GetMaterial _mesh 0) "None" :!class /Script/Engine.PrimitiveComponent))
      (bind _returnvalue_3 (Rendering|Material|GetVectorParameterValue _returnvalue_2 "DissolveEdgeColor" :!class /Script/Engine.MaterialInstanceDynamic))
      (Niagara|SetNiagaraVariable(LinearColor) (Variables|Default|GetNiagaraSystem) "DissolveParticleColor" _returnvalue_3))))

(event Custom|RemoveHealthBar
  (Class|EnemyUIComponent|RemoveEnemyDrawnWidgetsifAny (Variables|Default|GetEnemyUI_Component)))

(event Custom|HandleEntryFX
  (bind _enemycombatcomponent (Variables|Default|GetEnemyCombatComponent))
  (bind _returnvalue (Class|PawnCombatComponent|GetCharacterCurrentEquippedWeapon _enemycombatcomponent))
  (Components|Timeline|SetPlayRate (Variables|Default|GetEntryRestoreTimeline) (/ 1.0 (Variables|Default|GetTotalEntryRestoreTime)))
  (bind _normalizedfloattrack (Timeline|EntryRestoreTimeline ReverseFromEnd)
    (:Update
      (bind _output_get (Variables|Default|SetRestoreFloatTrack _normalizedfloattrack))
      (Rendering|Material|SetScalarParameterValueonMaterials (Variables|Character|GetMesh) "DissolveAmount" _output_get)
      (Utilities|IsValid _returnvalue
        (:Is%20Valid
          (Rendering|Material|SetScalarParameterValueonMaterials (Variables|/Script/Goliath.GoliathWeaponBase|GetWeaponMesh _returnvalue) "DissolveAmount" (Variables|Default|GetRestoreFloatTrack)))))))

(event Custom|HandleEntryMontage
  (bind _entrymontagestoplay (Variables|Default|GetEntryMontagesToPlay))
  (if (Utilities|Array|IsNotEmpty _entrymontagestoplay)
    (Animation|PlayAnimMontage (.OutItem (Utilities|Array|Random _entrymontagestoplay)) 1.0 "None")))

(event EventBeginPlay
  (CallFunction|HandleEntryFX)
  (CallFunction|HandleEntryMontage))

(event EventOnEnemyDied
  (params (DissolveNiagaraSystem :type Niagara%20System%20Soft%20Object%20Reference))
  (Variables|Default|SetCurrentEquippedWeapon (Class|PawnCombatComponent|GetCharacterCurrentEquippedWeapon (Variables|Default|GetEnemyCombatComponent)))
  (CallFunction|DsiableAnimations)
  (CallFunction|RemoveHealthBar)
  (CallFunction|SpawnVFXEffects DissolveNiagaraSystem)
  (CallFunction|SpawnVFXMaterial))

(fn ConstructionScript)